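; BP_Tube is a possessable, physics-driven water slide tube that the player rides from a character and exits once slowed or stopped.
; Enhanced Input applies forces and torque, while Tick drives speed-based audio, noise-modulated force feedback, braking and buoyancy.
; Overlapping a BP_Water_Slide RunOutVolume starts braking or floating, plays splash effects and optionally spawns a replacement tube at the start.
; Timelines blend the camera between character and tube on possession and exit.
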(event OnComponentBeginOverlap(Collision)
  (params (OverlappedComponent :type Primitive%20Component%20Object%20Reference) (OtherActor :type Actor%20Object%20Reference) (OtherComp :type Primitive%20Component%20Object%20Reference) (OtherBodyIndex :type Integer) (bFromSweep :type Boolean) (SweepResult :type Hit%20Result%20Structure%20%28by%20ref%29))
  (bind _sphere (Variables|Default|GetSphere))
  ;[1 1 1] Fall out of Water Slide
  (if (and (Utilities|String|Contains (Utilities|GetDisplayName OtherComp) "RunOutVolume") (not (Variables|Default|GetBraking%20in%20Water)))
    (bind _asbp_water_slide (Utilities|Casting|CastToBP_Water_Slide OtherActor))
    (Utilities|FlowControl|DoOnce false
      (:Completed
        (Variables|FloatingAfterFinish|SetPool%20Water%20Height (Variables|/Game/Water_Slide_System/Blueprints/BP_Water_Slide.BP_Water_Slide_C|GetPool%20Water%20height _asbp_water_slide))
        (Variables|FloatingafterFinish|SetFloat%20on%20Water (not (Variables|/Game/Water_Slide_System/Blueprints/BP_Water_Slide.BP_Water_Slide_C|GetRunout _asbp_water_slide)))
        (Variables|Default|SetBraking%20in%20Water true)
        (Audio|PlaySoundatLocation "/Game/Water_Slide_System/Sound/CUE/SC_Jump_In_Water.SC_Jump_In_Water" (Transformation|GetActorLocation) "0, 0, 0" 8.0 1.0 0.0 "/Game/Water_Slide_System/Sound/ATT_Waterfall.ATT_Waterfall" 0 0 0)
        (Utilities|FlowControl|Sequence
          (:then_0
            ;;[1 1 1] Force Feedback
            (if (and (Variables|Tube|GetForce%20Feedback) (Variables|Default|GetIs%20Possessed))
              (Game|Feedback|ClientPlayForceFeedback (Game|GetPlayerController 0) "/Game/Water_Slide_System/Blueprints/Additional/Fall_in_Water.Fall_in_Water" "None" false false false)))
          (:then_1
            (CallFunction|SpawnNewTubeatStart))
          (:then_2
            (Components|Activation|Activate (Variables|Default|GetSplashes) false))
          (:then_3
            (Rendering|Material|SetScalarParameterValueonMaterials (Variables|Default|GetTube%20Mesh) "Drops Amount" 1.0)
            (Transformation|DetachFromComponent _sphere "KeepRelative" "KeepRelative" "KeepRelative" true)
            (Components|DestroyComponent _sphere)))))))

(event Input|EnhancedActionEvents|EnhancedInputActionIA_Exit
  (params (ActionValue :type Boolean) (ElapsedSeconds :type Float%20%28double-precision%29) (TriggeredSeconds :type Float%20%28double-precision%29) (InputAction :type Input%20Action%20Object%20Reference :default "/Game/Water_Slide_System/Blueprints/Additional/Input/Actions/IA_Exit.IA_Exit"))
  (bind _returnvalue (Utilities|Time|GetWorldDeltaSeconds))
  (bind _camera (Variables|Default|GetCamera))
  (bind _character (Variables|Default|GetCharacter))
  (bind _collision (Variables|Default|GetCollision))
  (bind _returnvalue_2 (Transformation|GetWorldTransform _camera))
  (bind _returnvalue_3 (Actor|GetComponentsByClass _character "/Script/Engine.CameraComponent"))
  (bind _output (Utilities|Array|Get(acopy) _returnvalue_3))
  (bind _returnvalue_4 (Transformation|GetWorldTransform _output))
  ;[1 1 1] Exit Tube
  (if (Variables|Default|GetTime%20to%20Exit)
    (if (Variables|Default|GetIs%20Possessed)
      (Utilities|FlowControl|DoOnce false
        (:Completed
          (Variables|Default|SetTube%20Used true)
          (Components|DestroyComponent (Variables|Default|GetS_Speeding_Wind))
          (Rendering|SetVisibility (Variables|Default|GetE_Key_Widget) false false)
          (Transformation|SetActorLocationAndRotation (Variables|Default|GetCharacter) (+ (Transformation|GetWorldLocation _collision) (* (Math|Vector|GetRightVector _collision) 2e+02 (Math|Float|SelectFloat -1.0 1.0 (Variables|EndOfRide|GetExit%20to%20Left))) "0.000000,0.000000,50.000000") (Math|Rotator|MakeRotator 0.0 0.0 (.yaw (Math|Rotator|CombineRotators (Transformation|GetWorldRotation _collision) (Math|Rotator|MakeRotator 0.0 0.0 (Math|Float|SelectFloat 45.0 -45.0 (Variables|EndOfRide|GetExit%20to%20Left)))))))
          (Widget|SetVisibility (Variables|Default|GetHUD) "Hidden" :!label _label)
          (Timeline|Timeline PlayFromStart
            (:Update
              (Transformation|SetWorldTransform _camera (Math|Transform|MakeTransform (Math|Interpolation|VInterpTo (.location _returnvalue_2) (.location _returnvalue_4) _returnvalue 5.0) (Math|Interpolation|RInterpTo (.rotation _returnvalue_2) (Math|Rotator|MakeRotator 0.0 0.0 (.yaw (.rotation _returnvalue_4))) _returnvalue 5.0) "1.000000,1.000000,1.000000") false false)
              (Camera|SetFieldOfView _camera (Math|Interpolation|FInterpTo (Variables|/Script/Engine.CameraComponent|GetFieldOfView _camera) 9e+01 _returnvalue 5.0)))
            (:Finished
              (Input|DisableInput 0)
              (bind _aspawn (Utilities|Casting|CastToPawn _character))
              (Pawn|Possess (Game|GetPlayerController 0) _aspawn))))))
    (elif (Math|Boolean|ANDBoolean (Variables|EndofRide|GetCan%20be%20exited%20any%20time%20when%20stopped) (Variables|Default|GetAllow%20exit%20at%20any%20time) (Variables|Default|GetIs%20Possessed) (< (Variables|Default|GetCurrent%20Velocity) 1e+02))
      (Variables|Default|SetAllow%20exit%20at%20any%20time false)
      (Variables|Default|SetIs%20Possessed false)
      (goto _label))))

(event Input|EnhancedActionEvents|EnhancedInputActionIA_Tube_Move
  (params (ActionValue :type Vector%202D%20Structure) (ElapsedSeconds :type Float%20%28double-precision%29) (TriggeredSeconds :type Float%20%28double-precision%29) (InputAction :type Input%20Action%20Object%20Reference :default "/Game/Water_Slide_System/Blueprints/Additional/Input/Actions/IA_Tube_Move.IA_Tube_Move"))
  (bind _returnvalue (Math|Float|MakeLiteralFloat 8e+03))
  (bind _collision (Variables|Default|GetCollision))
  ;[1 1 1] Move input
  (Physics|AddForce _collision (+ (* (Math|Vector|GetForwardVector _collision) (Math|Float|SelectFloat (Math|Float|Clamp(Float) (.y ActionValue) -1.0 0.0) (.y ActionValue) (> (Math|Vector|VectorLength (Transformation|GetComponentVelocity _collision)) 1.5e+02)) _returnvalue) (* (Math|Vector|GetRightVector _collision) (.x ActionValue) _returnvalue 3.0)) "None" false))

(event Input|EnhancedActionEvents|EnhancedInputActionIA_Tube_Look
  (params (ActionValue :type Vector%202D%20Structure) (ElapsedSeconds :type Float%20%28double-precision%29) (TriggeredSeconds :type Float%20%28double-precision%29) (InputAction :type Input%20Action%20Object%20Reference :default "/Game/Water_Slide_System/Blueprints/Additional/Input/Actions/IA_Tube_Look.IA_Tube_Look"))
  (bind _returnvalue (* (.y ActionValue) -1.5))
  (bind _returnvalue_2 (* (.x ActionValue) 1.5))
  (bind _camera (Variables|Default|GetCamera))
  (bind _returnvalue_3 (Math|Rotator|MakeRotator 0.0 _returnvalue _returnvalue_2))
  (bind _relativerotation (Variables|/Script/Engine.SceneComponent|GetRelativeRotation _camera))
  (bind _returnvalue_4 (Math|Rotator|CombineRotators _relativerotation _returnvalue_3))
  ;[1 1 1] Camera Rotation
  (Utilities|FlowControl|Sequence
    (:then_0
      (Transformation|SetRelativeRotation _camera (Math|Rotator|MakeRotator 0.0 (Math|Float|Clamp(Float) (.pitch _returnvalue_4) -5e+01 5e+01) (Math|Float|Clamp(Float) (.yaw _returnvalue_4) -5e+01 5e+01)) false false))
    (:then_1
      ;[1 1 1] Rotate Tube
      (Class|PrimitiveComponent|AddTorqueinRadians (Variables|Default|GetCollision) (Math|Vector|MakeVector 0.0 0.0 (* (.x ActionValue) 2e+05)) "None" false))))

(event EventBeginPlay
  ;[1 1 1] Begin Play
  (Collision|SetCollisionEnabled (Variables|Default|GetSphere) "NoCollision")
  (if (Variables|EndOfRide|GetSpawn%20new%20Tube%20at%20Starting%20Location)
    (Variables|Default|SetStarting%20Location (Transformation|GetActorTransform))))

(event EventPossessed
  (params (NewController :type Controller%20Object%20Reference))
  (bind _returnvalue (Utilities|Time|GetWorldDeltaSeconds))
  (bind _camera (Variables|Default|GetCamera))
  (bind _camera_2 (Variables|Default|GetCamera))
  (bind _character (Variables|Default|GetCharacter))
  (bind _collision (Variables|Default|GetCollision))
  (bind _returnvalue_2 (Transformation|GetRelativeTransform _camera_2))
  (bind _returnvalue_3 (Actor|GetComponentsByClass _character "/Script/Engine.CameraComponent"))
  (bind _output (Utilities|Array|Get(acopy) _returnvalue_3))
  ;[1 1 1] Possession
  (Utilities|FlowControl|DelayUntilNextTick)
  (Rendering|SetVisibility (Variables|Default|GetE_Key_Widget) false false)
  (if (== (Pawn|GetControlledPawn (Game|GetPlayerController 0)) self)
    (Variables|Default|SetIs%20Possessed true)
    (Collision|SetCollisionEnabled (Variables|Default|GetSphere) "QueryAndPhysics")
    (Utilities|FlowControl|Sequence
      (:then_0
        (bind _returnvalue_4 (UserInterface|CreateWidget "/Game/Water_Slide_System/Blueprints/Additional/HUD_Tube.HUD_Tube_C"))
        (bind _output_get (Variables|Default|SetHUD _returnvalue_4))
        (UserInterface|Viewport|AddtoViewport _output_get 0))
      (:then_1
        (bind _asplayer_controller (Utilities|Casting|CastToPlayerController NewController))
        (Utilities|IsValid (PlayerController|LocalPlayerSubsystems|GetEnhancedInputLocalPlayerSubsystem _asplayer_controller)
          (:Is%20Valid
            (Input|AddMappingContext (PlayerController|LocalPlayerSubsystems|GetEnhancedInputLocalPlayerSubsystem _asplayer_controller) "/Game/Water_Slide_System/Blueprints/Additional/Input/IMC_Tube.IMC_Tube" 0 "(bIgnoreAllPressedKeysUntilRelease=True,bForceImmediately=False,bNotifyUserSettings=False)")
            ;;[1 1 1] Smooth camera transition from Character to Tube
            (if (Variables|Default|GetWas%20Possessed%20from%20Character)
              (Transformation|SetWorldTransform _camera (Transformation|GetWorldTransform _output) false false)
              (Camera|SetFieldOfView _camera (Variables|/Script/Engine.CameraComponent|GetFieldOfView _output))
              (Timeline|Camera%20Transition PlayFromStart
                (:Update
                  (Transformation|SetRelativeTransform _camera_2 (Math|Transform|MakeTransform (Math|Interpolation|VInterpTo (.location _returnvalue_2) "0.000000,0.000000,25.000000" _returnvalue 3.0) (Math|Interpolation|RInterpTo (.rotation _returnvalue_2) "0, 0, 0" _returnvalue 3.0) "1.000000,1.000000,1.000000") false false)
                  (Camera|SetFieldOfView _camera_2 (Math|Interpolation|FInterpTo (Variables|/Script/Engine.CameraComponent|GetFieldOfView _camera_2) (Variables|Tube|GetCamera%20FOV) _returnvalue 3.0))))))))
      (:then_3
        ;;[1 1 1] Allow Exit at any time
        (if (Variables|EndofRide|GetCan%20be%20exited%20any%20time%20when%20stopped)
          (Input|EnableInput 0)
          (Utilities|FlowControl|Delay 0.5)
          (Variables|Default|SetAllow%20exit%20at%20any%20time true)))
      (:then_4
        (if (Variables|Tube|GetAuto%20Launch%20when%20possessed)
          (Timeline|Start PlayFromStart
            (:Update
              (Physics|AddForce _collision (* (Math|Vector|GetForwardVector _collision) (Math|Float|MakeLiteralFloat 8e+03)) "None" false))))))))

(event EventTick
  (params (DeltaSeconds :type Float%20%28single-precision%29))
  (bind _returnvalue (Game|GetPlayerController 0))
  (bind _returnvalue_2 (Utilities|Time|GetWorldDeltaSeconds))
  (bind _hud (Variables|Default|GetHUD))
  (bind _force (Variables|FloatingAfterFinish|GetForce))
  (bind _collision (Variables|Default|GetCollision))
  (bind _collision_2 (Variables|Default|GetCollision))
  (bind _pool_water_height (Variables|FloatingAfterFinish|GetPool%20Water%20Height))
  (bind _collision_3 (Variables|Default|GetCollision))
  (bind _collision_4 (Variables|Default|GetCollision))
  (bind _returnvalue_3 (Transformation|GetWorldLocation _collision_2))
  (bind _returnvalue_4 (Transformation|GetComponentVelocity _collision))
  (bind _returnvalue_5 (Transformation|GetComponentVelocity _collision_4))
  (bind _returnvalue_6 (- (.z _returnvalue_3) _pool_water_height))
  (bind _returnvalue_7 (Math|Float|MapRangeClamped _returnvalue_6 -2e+01 0.0 _force 0.0))
  (Utilities|FlowControl|Sequence
    (:then_0
      (if (not (Variables|Default|GetTube%20Used))
        (Utilities|FlowControl|Sequence
          (:then_0
            ;[1 1 1] Get Velocity
            (Variables|Default|SetCurrent%20Velocity (Math|Vector|VectorLength (Transformation|GetComponentVelocity (Variables|Default|GetCollision))))
            ;[1 1 1] Braking
            (if (Variables|Default|GetBraking%20in%20Water)
              (Physics|AddForce (Variables|Default|GetCollision) (* (Math|Vector|Normalize _returnvalue_4) (+ (Math|Vector|VectorLengthSquared _returnvalue_4) 5e+01) (Math|Float|SelectFloat -0.4 -0.2 (Variables|FloatingafterFinish|GetFloat%20on%20Water))) "None" false)))
          (:then_1
            ;[1 1 1] Sound
            (Audio|Components|Audio|SetVolumeMultiplier (Variables|Default|GetS_Speeding_Wind) (Math|Float|MapRangeClamped (Variables|Default|GetCurrent%20Velocity) 4e+02 1.2e+03 0.0 2.5) :!class /Script/Engine.AudioComponent)
            (Audio|Components|Audio|SetVolumeMultiplier (Variables|Default|GetWater_Flow) (Math|Float|MapRangeClamped (Variables|Default|GetCurrent%20Velocity) 1e+02 6e+02 0.5 (Math|Float|MapRangeClamped (Class|KismetMathLibrary|PerlinNoise1D (* (Utilities|Time|GetRealTimeSeconds) (Math|Float|MapRangeClamped (Variables|Default|GetCurrent%20Velocity) 2e+02 8e+02 1.5 4.0))) -1.0 1.0 0.2 2.0)) :!class /Script/Engine.AudioComponent)
            ;[1 1 1] Force Feedback
            (if (and (Variables|Default|GetIs%20Possessed) (Variables|Tube|GetForce%20Feedback))
              (Utilities|FlowControl|Sequence
                (:then_0
                  ;;[1 1 1] Calculate Acceleration
                  (Variables|Default|SetZ%20Acceleration (Math|Interpolation|FInterpTo (Variables|Default|GetZ%20Acceleration) (/ (- (.z _returnvalue_5) (Variables|Default|GetLast%20Z%20Velocity)) _returnvalue_2) _returnvalue_2 2e+01))
                  (Variables|Default|SetLast%20Z%20Velocity (.z _returnvalue_5)))
                (:then_1
                  (Game|Feedback|PlayDynamicForceFeedback _returnvalue (+ (* (Math|Float|MapRangeClamped (Class|KismetMathLibrary|PerlinNoise1D (Utilities|Time|GetRealTimeSeconds)) -1.0 1.0 0.0 1.0) -0.1) (Math|Float|MapRangeClamped (Variables|Default|GetCurrent%20Velocity) 1.5e+02 8e+02 -0.1 0.3) (Math|Float|Clamp(Float) (* (Math|Float|Absolute(Float) (.z (Math|Vector|GetRightVector (Variables|Default|GetCollision)))) 0.5) 0.0 0.4) (Math|Float|MapRangeClamped (Variables|Default|GetZ%20Acceleration) -5e+02 5e+02 -0.5 0.5)) -1.0 false true false true))
                (:then_2
                  (Game|Feedback|PlayDynamicForceFeedback _returnvalue (Math|Float|MapRangeClamped (Variables|Default|GetZ%20Acceleration) 3e+02 6e+02 0.0 0.25) -1.0 true false true false)))))
          (:then_2
            ;[1 1 1] Check if it is time to Exit (Tube speed < 1 m/s)
            (if (Math|Boolean|ANDBoolean (Variables|Default|GetWas%20Possessed%20from%20Character) (Variables|Default|GetBraking%20in%20Water) (not (Variables|Default|GetTime%20to%20Exit)))
              (if (< (Math|Vector|VectorLength (Transformation|GetComponentVelocity (Variables|Default|GetCollision))) 1e+02)
                (Variables|Default|SetTime%20to%20Exit true)
                (Utilities|IsValid _hud
                  (:Is%20Valid
                    (Variables|/Game/Water_Slide_System/Blueprints/Additional/HUD_Tube.HUD_Tube_C|SetExit _hud true))))))
          (:then_3
            ;[1 1 1] Camera Rotation
            (if (Variables|Default|GetIs%20Possessed)
              (bind _returnvalue_8 (Physics|GetPhysicsLinearVelocity (Variables|Default|GetCollision) "None")))))))
    (:then_4
      ;[1 1 1] Floating in Pool after landing
      (if (Variables|FloatingafterFinish|GetFloat%20on%20Water)
        (Utilities|FlowControl|Sequence
          (:then_0
            (Utilities|FlowControl|DoOnce false
              (:Completed
                (Class|PrimitiveComponent|SetAngularDamping (Variables|Default|GetCollision) 4.0))))
          (:then_1
            (bind _returnvalue_9 (Physics|GetPhysicsLinearVelocity _collision_3 "None"))
            (Physics|SetPhysicsLinearVelocity _collision_3 (Math|Vector|MakeVector (.x _returnvalue_9) (.y _returnvalue_9) (Math|Interpolation|FInterptoConstant (.z _returnvalue_9) 0.0 (Utilities|Time|GetWorldDeltaSeconds) 2e+02)) false "None")
            (if (> (Math|Float|Absolute(Float) _returnvalue_7) 2.0) ; When not disturbed, mesh physics will go to sleep
              (Class|PrimitiveComponent|AddForceatLocation (Variables|Default|GetCollision) (Math|Vector|MakeVector 0.0 0.0 _returnvalue_7) (+ (Transformation|GetActorLocation) (* (Math|Vector|GetUpVector (Variables|Default|GetCollision)) 5e+01)) "None"))))))))

(event Input|KeyboardEvents|S
  (params (Key :type Key%20Structure :default "None"))
  ;[1 1 1] Braking
)

(event Input|KeyboardEvents|D
  (params (Key :type Key%20Structure :default "None"))
  ;[1 1 1] Move input
)

(event Input|KeyboardEvents|A
  (params (Key :type Key%20Structure :default "None"))
  ;[1 1 1] Move input
)

(fn ConstructionScript
  (CallFunction|Customize)
  (if (Variables|Tube|GetAuto%20Launch%20when%20possessed)
    (Variables|EndofRide|SetCan%20be%20exited%20any%20time%20when%20stopped false)))

(fn PossessfromCharacter
  (params (Character :type Actor%20Object%20Reference))
  (Pawn|Possess (Game|GetPlayerController 0) self)
  (Variables|Default|SetCharacter Character)
  (Variables|Default|SetWas%20Possessed%20from%20Character true))

(fn Customize
  (bind _material (Variables|Tube|GetMaterial))
  (Camera|SetFieldOfView (Variables|Default|GetCamera) (Variables|Tube|GetCamera%20FOV))
  (Utilities|IsValid _material
    (:Is%20Valid
      (Rendering|Material|SetMaterial (Variables|Default|GetTube%20Mesh) 0 _material))))

(fn SpawnNewTubeatStart
  (if (Variables|EndOfRide|GetSpawn%20new%20Tube%20at%20Starting%20Location)
    (bind _returnvalue (Game|SpawnActorfromClass "BP_Tube_C" (Variables|Default|GetStarting%20Location) "AdjustIfPossibleButAlwaysSpawn" "MultiplyWithRoot" 0 0))
    (Variables|BP_Tube_C|SetMaterial _returnvalue (Variables|Tube|GetMaterial))
    (Variables|BP_Tube_C|SetCamera%20FOV _returnvalue (Variables|Tube|GetCamera%20FOV))
    (Variables|BP_Tube_C|SetSpawn%20new%20Tube%20at%20Starting%20Location _returnvalue (Variables|EndOfRide|GetSpawn%20new%20Tube%20at%20Starting%20Location))
    (Variables|BP_Tube_C|SetForce%20Feedback _returnvalue (Variables|Tube|GetForce%20Feedback))
    (Variables|BP_Tube_C|SetExit%20to%20Left _returnvalue (Variables|EndOfRide|GetExit%20to%20Left))
    (Variables|BP_Tube_C|SetCan%20be%20exited%20any%20time%20when%20stopped _returnvalue (Variables|EndofRide|GetCan%20be%20exited%20any%20time%20when%20stopped))
    (Variables|BP_Tube_C|SetAuto%20Launch%20when%20possessed _returnvalue (Variables|Tube|GetAuto%20Launch%20when%20possessed))
    (CallFunction|Customize _returnvalue)))