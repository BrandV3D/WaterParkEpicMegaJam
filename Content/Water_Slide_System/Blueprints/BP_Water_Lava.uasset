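; Spline-driven water slide actor that builds its flume, start piece, optional runout and end waterfall in the construction script.
; Spline mesh segments take alternating colors and per-section mesh and emissive overrides, while height-scaled pillars snap to the spline and reach down to a floor height.
; It also computes drop, slope and length readouts.
; TurnWaterON/OFF events drive a timeline that fades water through a material Visibility parameter.
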(event Custom|Turn%20Water%20OFF
  ;[1 1 1] Turn Water ON/OFF Events
  (if (Variables|Flume|GetWater%20Flowing)
    (Variables|Flume|SetWater%20Flowing false)
    (bind _visibility (Timeline|Timeline ReverseFromEnd)
      (:Update
        (CallFunction|SetWaterVisibility _visibility)))))

(event Custom|Turn%20Water%20ON
  ;[1 1 1] Turn Water ON/OFF Events
  (if (not (Variables|Flume|GetWater%20Flowing))
    (Variables|Flume|SetWater%20Flowing true)
    (bind _visibility (Timeline|Timeline PlayFromStart)
      (:Update
        (CallFunction|SetWaterVisibility _visibility)))))

(event EventBeginPlay)

(event Collision|EventActorBeginOverlap
  (params (OtherActor :type Actor%20Object%20Reference)))

(event EventTick
  (params (DeltaSeconds :type Float%20%28single-precision%29)))

(fn ConstructionScript
  (bind _alternating_colors_list (Variables|Flume|GetAlternating%20Colors%20List))
  (bind _color (Variables|Flume|GetColor))
  (bind _alternating_colors (Variables|Flume|GetAlternating%20Colors))
  (bind _output (Utilities|Array|Get(acopy) _alternating_colors_list))
  (bind _returnvalue (select _alternating_colors _output _color))
  (bind _returnvalue_2 (Math|Conversions|ToLinearColor(Color) _returnvalue))
  (bind _returnvalue_3 (Math|Conversions|ToVector(LinearColor) _returnvalue_2))
  (Utilities|FlowControl|Sequence
    (:then_0
      ;[1 1 1] Initialize
      (Variables|Default|SetSpline%20Length (Spline|GetSplineLength (Variables|Default|GetSpline)))
      (CallFunction|SetInfoVairables)
      ;[1 1 1] Set SM_Start mesh and Start safety
      (Transformation|AddLocalOffset (Variables|Default|GetSM_Start) (Spline|GetLocationatDistanceAlongSpline (Variables|Default|GetSpline) 0.0 "Local") false false)
      (Rendering|Material|SetVectorParameterValueonMaterials (Variables|Default|GetSM_Start) "Base Color" _returnvalue_3)
      (if (Variables|Flume|GetStart%20Safety)
        (bind _returnvalue_4 (AddComponent|AddStaticMeshComponent false))
        (Rendering|Material|SetVectorParameterValueonMaterials _returnvalue_4 "Base Color" _returnvalue_3)
        (Transformation|AttachComponentToComponent _returnvalue_4 (Variables|Default|GetSM_Start) "None" "KeepRelative" "KeepRelative" "KeepRelative" true)))
    (:then_1
      (CallFunction|AddFlumeMeshes)
      (CallFunction|AddRunout)
      (Pillars|AddPillars))
    (:then_2
      (CallFunction|SetWaterVisibility (Math|Conversions|ToFloat(Boolean) (Variables|Flume|GetWater%20Flowing))))))

(fn SetInfoVairables
  (bind _spline (Variables|Default|GetSpline))
  (bind _spline_2 (Variables|Default|GetSpline))
  (bind _spline_3 (Variables|Default|GetSpline))
  (bind _returnvalue (Spline|GetSplineLength _spline))
  (bind _returnvalue_2 (Spline|GetLocationatDistanceAlongSpline _spline 0.0 "World"))
  (bind _returnvalue_3 (Spline|GetSplineLength _spline_2))
  (bind _returnvalue_4 (Spline|GetLocationatDistanceAlongSpline _spline _returnvalue "World"))
  (bind _returnvalue_5 (/ _returnvalue_3 1e+02))
  (bind _returnvalue_6 (Math|Float|Ceil _returnvalue_5))
  (bind _returnvalue_7 (- (.z _returnvalue_2) (.z _returnvalue_4)))
  (bind _returnvalue_8 (/ _returnvalue_3 _returnvalue_6))
  (Utilities|FlowControl|Sequence
    (:then_0
      ;[1 1 1] Calculate Drop Height, Average Slope, Length
      (Variables|Info|SetDrop%20Height (Utilities|String|Append (Utilities|String|ToString(Float) (/ (Math|Float|Round (* _returnvalue_7 0.1)) 10)) " m"))
      (Variables|Info|SetAverage%20Slope (Utilities|String|Append (Utilities|String|ToString(Float) (/ (Math|Float|Round (Utilities|Operators|Divide _returnvalue_7 _returnvalue 0.001)) 10)) " %"))
      (Variables|Info|SetLength (Utilities|String|Append (Utilities|String|ToString(Float) (/ (Math|Float|Round (* _returnvalue 0.1)) 10)) " m")))
    (:then_1
      ;[1 1 1] Calculate Max Slope
      (LocalVariables|SetMaxSlope 0.0)
      (for _index (range 1 _returnvalue_6)
        (if (> (- (.z (Spline|GetLocationatDistanceAlongSpline _spline_3 (* (- _index 1) _returnvalue_8) "World")) (.z (Spline|GetLocationatDistanceAlongSpline _spline_3 (* _index _returnvalue_8) "World"))) (LocalVariables|GetMaxSlope))
          (LocalVariables|SetMaxSlope (- (.z (Spline|GetLocationatDistanceAlongSpline _spline_3 (* (- _index 1) _returnvalue_8) "World")) (.z (Spline|GetLocationatDistanceAlongSpline _spline_3 (* _index _returnvalue_8) "World"))))))
      (Variables|Info|SetMax%20Slope (Utilities|String|Append (Utilities|String|ToString(Float) (/ (Math|Float|Round (* (LocalVariables|GetMaxSlope) 1e+01)) 10)) " %")))))

(fn AddPillars
  (bind _returnvalue (Transformation|GetActorLocation))
  (bind _spline (Variables|Default|GetSpline))
  (bind _floor_height (Variables|Pillars|GetFloor%20Height))
  (bind _returnvalue_2 (- _floor_height (.z _returnvalue)))
  (if (not (Variables|Flume|GetSpline%20Edit%20Mode))
    (Utilities|FlowControl|Sequence
      (:then_0
        (Utilities|Array|Clear (Variables|Pillars|GetPillar%20Meshes)))
      (:then_1
        (for (_array_element _array_index) (Variables|Pillars|GetPillar)
          (bind _distance_on_spline (CallFunction|SearchNearestDistanceonSpline (Variables|Default|GetSpline) _array_element 2e+01))
          (Utilities|Array|SetArrayElem (Variables|Pillars|GetPillar) _array_index (Spline|GetLocationatDistanceAlongSpline _spline _distance_on_spline "Local")) ; Snap Widgets to Spline
          (bind _returnvalue_3 (AddComponent|AddStaticMeshComponent false (Math|Transform|MakeTransform (Spline|GetLocationatDistanceAlongSpline _spline _distance_on_spline "Local") (Math|Rotator|MakeRotator (.roll (Math|Conversions|RotationFromXVector (Spline|GetTangentatDistanceAlongSpline _spline _distance_on_spline "Local"))) (.pitch (Math|Conversions|RotationFromXVector (Spline|GetTangentatDistanceAlongSpline _spline _distance_on_spline "Local"))) (.yaw (Math|Conversions|RotationFromXVector (Spline|GetTangentatDistanceAlongSpline _spline _distance_on_spline "Local")))) "1.000000,1.000000,1.000000")))
          (Utilities|Array|Add (Variables|Pillars|GetPillar%20Meshes) _returnvalue_3)
          (if (> (- (.Z (Math|Vector|BreakVector (- (Spline|GetLocationatDistanceAlongSpline _spline _distance_on_spline "Local") (* (Math|Vector|Normalize (Math|Vector|ProjectVectorontoPlane (Class|SplineComponent|GetUpVectoratDistanceAlongSpline _spline _distance_on_spline "Local") (Math|Vector|Normalize (Math|Vector|CrossProduct "0.000000,0.000000,1.000000" (Spline|GetTangentatDistanceAlongSpline _spline _distance_on_spline "Local"))))) 68.0)))) _returnvalue_2) 0.0)
            (for _index (range 1 (Math|Integer|Clamp(Integer) (Math|Float|Round (/ (- (.Z (Math|Vector|BreakVector (- (Spline|GetLocationatDistanceAlongSpline _spline _distance_on_spline "Local") (* (Math|Vector|Normalize (Math|Vector|ProjectVectorontoPlane (Class|SplineComponent|GetUpVectoratDistanceAlongSpline _spline _distance_on_spline "Local") (Math|Vector|Normalize (Math|Vector|CrossProduct "0.000000,0.000000,1.000000" (Spline|GetTangentatDistanceAlongSpline _spline _distance_on_spline "Local"))))) 68.0)))) _returnvalue_2) (Math|Float|SelectFloat 4.5e+02 3e+02 (> (- (.Z (Math|Vector|BreakVector (- (Spline|GetLocationatDistanceAlongSpline _spline _distance_on_spline "Local") (* (Math|Vector|Normalize (Math|Vector|ProjectVectorontoPlane (Class|SplineComponent|GetUpVectoratDistanceAlongSpline _spline _distance_on_spline "Local") (Math|Vector|Normalize (Math|Vector|CrossProduct "0.000000,0.000000,1.000000" (Spline|GetTangentatDistanceAlongSpline _spline _distance_on_spline "Local"))))) 68.0)))) _returnvalue_2) 4e+02)))) 1 10))
              (bind _returnvalue_4 (AddComponent|AddStaticMeshComponent false (Math|Transform|MakeTransform (Math|Vector|MakeVector (.X (Math|Vector|BreakVector (- (Spline|GetLocationatDistanceAlongSpline _spline _distance_on_spline "Local") (* (Math|Vector|Normalize (Math|Vector|ProjectVectorontoPlane (Class|SplineComponent|GetUpVectoratDistanceAlongSpline _spline _distance_on_spline "Local") (Math|Vector|Normalize (Math|Vector|CrossProduct "0.000000,0.000000,1.000000" (Spline|GetTangentatDistanceAlongSpline _spline _distance_on_spline "Local"))))) 68.0)))) (.Y (Math|Vector|BreakVector (- (Spline|GetLocationatDistanceAlongSpline _spline _distance_on_spline "Local") (* (Math|Vector|Normalize (Math|Vector|ProjectVectorontoPlane (Class|SplineComponent|GetUpVectoratDistanceAlongSpline _spline _distance_on_spline "Local") (Math|Vector|Normalize (Math|Vector|CrossProduct "0.000000,0.000000,1.000000" (Spline|GetTangentatDistanceAlongSpline _spline _distance_on_spline "Local"))))) 68.0)))) (+ (* (/ (- _index 1) (Math|Integer|Clamp(Integer) (Math|Float|Round (/ (- (.Z (Math|Vector|BreakVector (- (Spline|GetLocationatDistanceAlongSpline _spline _distance_on_spline "Local") (* (Math|Vector|Normalize (Math|Vector|ProjectVectorontoPlane (Class|SplineComponent|GetUpVectoratDistanceAlongSpline _spline _distance_on_spline "Local") (Math|Vector|Normalize (Math|Vector|CrossProduct "0.000000,0.000000,1.000000" (Spline|GetTangentatDistanceAlongSpline _spline _distance_on_spline "Local"))))) 68.0)))) _returnvalue_2) (Math|Float|SelectFloat 4.5e+02 3e+02 (> (- (.Z (Math|Vector|BreakVector (- (Spline|GetLocationatDistanceAlongSpline _spline _distance_on_spline "Local") (* (Math|Vector|Normalize (Math|Vector|ProjectVectorontoPlane (Class|SplineComponent|GetUpVectoratDistanceAlongSpline _spline _distance_on_spline "Local") (Math|Vector|Normalize (Math|Vector|CrossProduct "0.000000,0.000000,1.000000" (Spline|GetTangentatDistanceAlongSpline _spline _distance_on_spline "Local"))))) 68.0)))) _returnvalue_2) 4e+02)))) 1 10)) (- (.Z (Math|Vector|BreakVector (- (Spline|GetLocationatDistanceAlongSpline _spline _distance_on_spline "Local") (* (Math|Vector|Normalize (Math|Vector|ProjectVectorontoPlane (Class|SplineComponent|GetUpVectoratDistanceAlongSpline _spline _distance_on_spline "Local") (Math|Vector|Normalize (Math|Vector|CrossProduct "0.000000,0.000000,1.000000" (Spline|GetTangentatDistanceAlongSpline _spline _distance_on_spline "Local"))))) 68.0)))) _returnvalue_2)) _returnvalue_2)) (Math|Rotator|MakeRotator 0.0 0.0 (.yaw (Math|Conversions|RotationFromXVector (Spline|GetTangentatDistanceAlongSpline _spline _distance_on_spline "Local")))) (Math|Vector|MakeVector (Math|Float|SelectFloat 1.5 1.0 (> (- (.Z (Math|Vector|BreakVector (- (Spline|GetLocationatDistanceAlongSpline _spline _distance_on_spline "Local") (* (Math|Vector|Normalize (Math|Vector|ProjectVectorontoPlane (Class|SplineComponent|GetUpVectoratDistanceAlongSpline _spline _distance_on_spline "Local") (Math|Vector|Normalize (Math|Vector|CrossProduct "0.000000,0.000000,1.000000" (Spline|GetTangentatDistanceAlongSpline _spline _distance_on_spline "Local"))))) 68.0)))) _returnvalue_2) 4e+02)) (Math|Float|SelectFloat 1.5 1.0 (> (- (.Z (Math|Vector|BreakVector (- (Spline|GetLocationatDistanceAlongSpline _spline _distance_on_spline "Local") (* (Math|Vector|Normalize (Math|Vector|ProjectVectorontoPlane (Class|SplineComponent|GetUpVectoratDistanceAlongSpline _spline _distance_on_spline "Local") (Math|Vector|Normalize (Math|Vector|CrossProduct "0.000000,0.000000,1.000000" (Spline|GetTangentatDistanceAlongSpline _spline _distance_on_spline "Local"))))) 68.0)))) _returnvalue_2) 4e+02)) (* (Utilities|Operators|Divide (- (.Z (Math|Vector|BreakVector (- (Spline|GetLocationatDistanceAlongSpline _spline _distance_on_spline "Local") (* (Math|Vector|Normalize (Math|Vector|ProjectVectorontoPlane (Class|SplineComponent|GetUpVectoratDistanceAlongSpline _spline _distance_on_spline "Local") (Math|Vector|Normalize (Math|Vector|CrossProduct "0.000000,0.000000,1.000000" (Spline|GetTangentatDistanceAlongSpline _spline _distance_on_spline "Local"))))) 68.0)))) _returnvalue_2) (Math|Float|SelectFloat 4.5e+02 3e+02 (> (- (.Z (Math|Vector|BreakVector (- (Spline|GetLocationatDistanceAlongSpline _spline _distance_on_spline "Local") (* (Math|Vector|Normalize (Math|Vector|ProjectVectorontoPlane (Class|SplineComponent|GetUpVectoratDistanceAlongSpline _spline _distance_on_spline "Local") (Math|Vector|Normalize (Math|Vector|CrossProduct "0.000000,0.000000,1.000000" (Spline|GetTangentatDistanceAlongSpline _spline _distance_on_spline "Local"))))) 68.0)))) _returnvalue_2) 4e+02)) (Math|Integer|Clamp(Integer) (Math|Float|Round (/ (- (.Z (Math|Vector|BreakVector (- (Spline|GetLocationatDistanceAlongSpline _spline _distance_on_spline "Local") (* (Math|Vector|Normalize (Math|Vector|ProjectVectorontoPlane (Class|SplineComponent|GetUpVectoratDistanceAlongSpline _spline _distance_on_spline "Local") (Math|Vector|Normalize (Math|Vector|CrossProduct "0.000000,0.000000,1.000000" (Spline|GetTangentatDistanceAlongSpline _spline _distance_on_spline "Local"))))) 68.0)))) _returnvalue_2) (Math|Float|SelectFloat 4.5e+02 3e+02 (> (- (.Z (Math|Vector|BreakVector (- (Spline|GetLocationatDistanceAlongSpline _spline _distance_on_spline "Local") (* (Math|Vector|Normalize (Math|Vector|ProjectVectorontoPlane (Class|SplineComponent|GetUpVectoratDistanceAlongSpline _spline _distance_on_spline "Local") (Math|Vector|Normalize (Math|Vector|CrossProduct "0.000000,0.000000,1.000000" (Spline|GetTangentatDistanceAlongSpline _spline _distance_on_spline "Local"))))) 68.0)))) _returnvalue_2) 4e+02)))) 1 10)) (Math|Float|SelectFloat 1.5 1.0 (> (- (.Z (Math|Vector|BreakVector (- (Spline|GetLocationatDistanceAlongSpline _spline _distance_on_spline "Local") (* (Math|Vector|Normalize (Math|Vector|ProjectVectorontoPlane (Class|SplineComponent|GetUpVectoratDistanceAlongSpline _spline _distance_on_spline "Local") (Math|Vector|Normalize (Math|Vector|CrossProduct "0.000000,0.000000,1.000000" (Spline|GetTangentatDistanceAlongSpline _spline _distance_on_spline "Local"))))) 68.0)))) _returnvalue_2) 4e+02)))))))
              (Utilities|Array|Add (Variables|Pillars|GetPillar%20Meshes) _returnvalue_4))))
        (for _array_element_2 (Variables|Pillars|GetPillar%20Meshes)
          (Rendering|Material|SetVectorParameterValueonMaterials _array_element_2 "Base Color" (Math|Conversions|ToVector(LinearColor) (Math|Conversions|ToLinearColor(Color) (Variables|Pillars|GetPillars%20Color)))))))))

(fn SpacePillarsEvenly
  (bind _pillar_spacing__m_ (Variables|Pillars|GetPillar%20Spacing%20%28m%29))
  (bind _spline_length (Variables|Default|GetSpline%20Length))
  (bind _returnvalue (Utilities|Operators|Divide _spline_length _pillar_spacing__m_ 1e+02))
  (bind _returnvalue_2 (Math|Float|Floor _returnvalue))
  (Utilities|FlowControl|Sequence
    (:then_0
      ;[1 1 1] Clear Pillar array and fill it with locations of evenly spaced Pillars
      (Utilities|Array|Clear (Variables|Pillars|GetPillar))
      (for _index (range 1 _returnvalue_2)
        (Utilities|Array|Add (Variables|Pillars|GetPillar) (Spline|GetLocationatDistanceAlongSpline (Variables|Default|GetSpline) (* (Variables|Default|GetSpline%20Length) (/ (- (Math|Conversions|ToFloat(Integer) _index) 0.5) (Math|Conversions|ToFloat(Integer) _returnvalue_2))) "Local"))))
    (:then_1
      ;[1 1 1] Destroy all Pillars and add new Pillars according to new Pillars array
      (for _array_element (Variables|Pillars|GetPillar%20Meshes)
        (Components|DestroyComponent _array_element))
      (Pillars|AddPillars))))

(fn ChangeSectionsTypes
  (params (Section%20Mesh :type Spline%20Mesh%20Component%20Object%20Reference) (Section%20# :type Integer))
  (bind _default_mesh (Variables|Flume|GetDefault%20Mesh))
  ;[1 1 1] Set Max Close Index (closest index to take Section Type parameters)
  (LocalVariables|SetMax%20Close%20index -1)
  (bind (_array_element _array_index) (Utilities|Array|ForEachLoopwithBreak (Variables|Flume|GetSections%20Type%20List))
    (:LoopBody
      (if (and (> Section%20# (.segmentfromstart _array_element)) (>= (.segmentfromstart _array_element) (LocalVariables|GetMax%20Close%20index)))
        (LocalVariables|SetMax%20Close%20index _array_index)))
    (:Completed
      (if (> (LocalVariables|GetMax%20Close%20index) -1)
        (Utilities|FlowControl|Sequence
          (:then_0
            (Components|StaticMesh|SetStaticMesh Section%20Mesh (.Value (Utilities|Map|Find (Variables|Default|GetSection%20Types) (.mesh (Utilities|Array|Get(acopy) (Variables|Flume|GetSections%20Type%20List) (LocalVariables|GetMax%20Close%20index))))))
            (Rendering|Material|SetScalarParameterValueonMaterials Section%20Mesh "Emissive Intensity" (* (Math|Conversions|ToFloat(Boolean) (.emissivelights (Utilities|Array|Get(acopy) (Variables|Flume|GetSections%20Type%20List) (LocalVariables|GetMax%20Close%20index)))) 5.0))
            (Rendering|Material|SetScalarParameterValueonMaterials Section%20Mesh "Emissive Running" (Math|Conversions|ToFloat(Boolean) (.emissiverunning (Utilities|Array|Get(acopy) (Variables|Flume|GetSections%20Type%20List) (LocalVariables|GetMax%20Close%20index)))))
            (Rendering|Material|SetScalarParameterValueonMaterials Section%20Mesh "Emissive Rainbow" (Math|Conversions|ToFloat(Boolean) (.emissiverainbow (Utilities|Array|Get(acopy) (Variables|Flume|GetSections%20Type%20List) (LocalVariables|GetMax%20Close%20index)))))
            (Rendering|Material|SetVectorParameterValueonMaterials Section%20Mesh "Emissive Color" (Math|Conversions|ToVector(LinearColor) (Math|Conversions|ToLinearColor(Color) (.emissivecolor (Utilities|Array|Get(acopy) (Variables|Flume|GetSections%20Type%20List) (LocalVariables|GetMax%20Close%20index))))))
            (if (Utilities|Enum|Equal(Enum) (.mesh (Utilities|Array|Get(acopy) (Variables|Flume|GetSections%20Type%20List) (LocalVariables|GetMax%20Close%20index))) "NewEnumerator2")
              (Rendering|Material|SetScalarParameterValueonMaterials Section%20Mesh "AO" 0.04)))
          (:then_1
            (if (.usecolor (Utilities|Array|Get(acopy) (Variables|Flume|GetSections%20Type%20List) (LocalVariables|GetMax%20Close%20index)))
              (Rendering|Material|SetVectorParameterValueonMaterials Section%20Mesh "Base Color" (Math|Conversions|ToVector(LinearColor) (Math|Conversions|ToLinearColor(Color) (.color (Utilities|Array|Get(acopy) (Variables|Flume|GetSections%20Type%20List) (LocalVariables|GetMax%20Close%20index)))))))))
        (else
          (Components|StaticMesh|SetStaticMesh Section%20Mesh (.Value (Utilities|Map|Find (Variables|Default|GetSection%20Types) _default_mesh)))
          (if (Utilities|Enum|Equal(Enum) _default_mesh "NewEnumerator2")
            (Rendering|Material|SetScalarParameterValueonMaterials Section%20Mesh "AO" 0.04)))))))

(fn AddFlumeMeshes
  (bind _alternating_colors_list (Variables|Flume|GetAlternating%20Colors%20List))
  (bind _spline (Variables|Default|GetSpline))
  (bind _mesh_length (Variables|Default|GetMesh%20Length))
  (if (not (Variables|Flume|GetSpline%20Edit%20Mode))
    (bind _output_get (Variables|Info|SetNumber%20of%20Segments (Math|Float|Round (/ (Variables|Default|GetSpline%20Length) (Variables|Default|GetMesh%20Length)))))
    (for _index (range 1 _output_get)
      (bind _returnvalue (AddComponent|AddSplineMeshComponent false))
      (Rendering|Material|SetScalarParameterValueonMaterials _returnvalue "Emissive Intensity" 0.0)
      (SplineMesh|SetStartandEnd _returnvalue (Spline|GetLocationatDistanceAlongSpline _spline (* (/ (Variables|Default|GetSpline%20Length) (Variables|Info|GetNumber%20of%20Segments)) (- _index 1)) "Local") (Math|Vector|SelectVector "400.000000,0.000000,0.000000" (* (Math|Vector|Normalize (Spline|GetTangentatDistanceAlongSpline _spline (* (/ (Variables|Default|GetSpline%20Length) (Variables|Info|GetNumber%20of%20Segments)) (- _index 1)) "Local")) _mesh_length) (== _index 1)) (Spline|GetLocationatDistanceAlongSpline _spline (* (/ (Variables|Default|GetSpline%20Length) (Variables|Info|GetNumber%20of%20Segments)) _index) "Local") (* _mesh_length (Math|Vector|Normalize (Spline|GetTangentatDistanceAlongSpline _spline (* (/ (Variables|Default|GetSpline%20Length) (Variables|Info|GetNumber%20of%20Segments)) _index) "Local"))) true :!class /Script/Engine.SplineMeshComponent)
      (Utilities|FlowControl|Sequence
        (:then_0
          (Class|SplineMeshComponent|SetStartRoll _returnvalue (Math|Trig|DegreesToRadians (Class|SplineComponent|GetRollatDistanceAlongSpline _spline (* (/ (Variables|Default|GetSpline%20Length) (Variables|Info|GetNumber%20of%20Segments)) (- _index 1)) "Local")) true)
          (Class|SplineMeshComponent|SetEndRoll _returnvalue (Math|Trig|DegreesToRadians (Class|SplineComponent|GetRollatDistanceAlongSpline _spline (* (/ (Variables|Default|GetSpline%20Length) (Variables|Info|GetNumber%20of%20Segments)) _index) "Local")) true)
          (Utilities|Array|Add (Variables|Flume|GetFlume%20Meshes) _returnvalue))
        (:then_1
          ;[1 1 1] Change Flume Color
          (Rendering|Material|SetVectorParameterValueonMaterials _returnvalue "Base Color" (Math|Conversions|ToVector(LinearColor) (Math|Conversions|ToLinearColor(Color) (select (Variables|Flume|GetAlternating%20Colors) (Utilities|Array|Get(acopy) _alternating_colors_list (Math|Integer|%(Integer) _index (Utilities|Array|Length _alternating_colors_list))) (Variables|Flume|GetColor))))))
        (:then_2
          (CallFunction|ChangeSectionsTypes _returnvalue _index))))))

(fn AddRunout
  (bind _spline (Variables|Default|GetSpline))
  (bind _runout_height_offset (Variables|EndofSlide|GetRunout%20Height%20Offset))
  (bind _spline_length (Variables|Default|GetSpline%20Length))
  (bind _returnvalue (Spline|GetLocationatDistanceAlongSpline _spline _spline_length "Local"))
  (bind _returnvalue_2 (Spline|GetTangentatDistanceAlongSpline _spline _spline_length "Local"))
  (bind _returnvalue_3 (Math|Vector|Normalize _returnvalue_2))
  (bind _returnvalue_4 (+ _returnvalue (Math|Vector|MakeVector 0.0 0.0 _runout_height_offset)))
  (bind _returnvalue_5 (* _returnvalue_3 "1.000000,1.000000,0.000000"))
  (bind _returnvalue_6 (* _returnvalue_5 3e+02))
  (bind _returnvalue_7 (+ _returnvalue_4 "0.000000,0.000000,-85.000000" _returnvalue_6))
  (Utilities|FlowControl|Sequence
    (:then_0
      (if (Variables|EndofSlide|GetRunout)
        (bind _returnvalue_8 (AddComponent|AddStaticMeshComponent false (Math|Transform|MakeTransform _returnvalue_4 (Math|Rotator|MakeRotator 0.0 0.0 (.yaw (Math|Conversions|RotationFromXVector _returnvalue_2))) "1.000000,1.000000,1.000000")))
        ;[1 1 1] Runout Color
        (Rendering|Material|SetVectorParameterValueonMaterials _returnvalue_8 "Base Color" (Math|Conversions|ToVector(LinearColor) (Math|Conversions|ToLinearColor(Color) (select (Variables|Flume|GetAlternating%20Colors) (Utilities|Array|Get(acopy) (Variables|Flume|GetAlternating%20Colors%20List)) (Variables|Flume|GetColor)))))))
    (:then_1
      ;[1 1 1] Position RunOutVolume
      (Transformation|SetRelativeTransform (Variables|Default|GetRunOutVolume) (Math|Transform|MakeTransform (Math|Vector|MakeVector (.x _returnvalue_7) (.y _returnvalue_7) (Math|Float|SelectFloat (.z _returnvalue_7) (.z (Math|Transform|InverseTransformLocation (Transformation|GetActorTransform) (Math|Vector|MakeVector 0.0 0.0 (- (Variables|EndOfSlide|GetPool%20Water%20height) 2e+01)))) (Variables|EndofSlide|GetRunout))) (Math|Rotator|MakeRotator 0.0 0.0 (.yaw (Math|Conversions|RotationFromXVector _returnvalue_2))) "1.000000,1.000000,1.000000") false false))
    (:then_2
      ;[1 1 1] Add Waterfall at the End
      (if (and (Variables|EndOfSlide|GetWaterfall%20at%20the%20End) (not (Variables|Flume|GetSpline%20Edit%20Mode)))
        (bind _returnvalue_9 (AddComponent|AddStaticMeshComponent false (Math|Transform|MakeTransform _returnvalue (Math|Conversions|RotationFromXVector _returnvalue_2) "1.000000,1.000000,1.000000")))
        (Variables|EndOfSlide|SetWaterfall%20mesh _returnvalue_9)))))

(fn SearchNearestDistanceonSpline
  (params (Spline :type Spline%20Component%20Object%20Reference) (Location :type Vector) (Spline%20Segment%20Length%20%28cm%29 :type Float%20%28double-precision%29))
  (LocalVariables|SetSegmentLength Spline%20Segment%20Length%20%28cm%29)
  (LocalVariables|SetMinDistance (Math|Vector|VectorLength (- Location (Spline|GetLocationatDistanceAlongSpline Spline 0.0 "Local"))))
  (for _index (range 1 (Math|Float|Truncate (/ (Spline|GetSplineLength Spline) Spline%20Segment%20Length%20%28cm%29)))
    (if (< (Math|Vector|VectorLength (- Location (Spline|GetLocationatDistanceAlongSpline Spline (* _index (LocalVariables|GetSegmentLength)) "Local"))) (LocalVariables|GetMinDistance))
      (LocalVariables|SetMinDistance (Math|Vector|VectorLength (- Location (Spline|GetLocationatDistanceAlongSpline Spline (* _index (LocalVariables|GetSegmentLength)) "Local"))))
      (LocalVariables|SetPositition%20Index _index)))
  (return (* (LocalVariables|GetPositition%20Index) (LocalVariables|GetSegmentLength)) (LocalVariables|GetMinDistance)))

(fn SetWaterVisibility
  (params (Visibility :type Float%20%28single-precision%29))
  (for _array_element (Variables|Flume|GetFlume%20Meshes)
    (Rendering|Material|SetScalarParameterValueonMaterials _array_element "Visibility" Visibility))
  (Rendering|Material|SetScalarParameterValueonMaterials (Variables|Default|GetSM_Start) "Visibility" Visibility)
  (if (Variables|EndOfSlide|GetWaterfall%20at%20the%20End)
    (Rendering|Material|SetScalarParameterValueonMaterials (Variables|Default|GetSM_Start) "Visibility" Visibility)
    (Rendering|SetVisibility (Variables|EndOfSlide|GetWaterfall%20mesh) (> Visibility 0.0) false)))