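; Procedural rectangular pool actor for the water slide system, built entirely in the Construction Script from size and depth variables.
; It places mirrored or rotated corners and stretched 200-unit wall segments, applies wall and coping materials, then adds a scaled bottom and optional water surface.
; Ladders map 0–100 perimeter positions onto edge transforms, and a downward trace picks 3- or 5-step meshes by local depth.
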(event EventBeginPlay)

(event Collision|EventActorBeginOverlap
  (params (OtherActor :type Actor%20Object%20Reference)))

(event EventTick
  (params (DeltaSeconds :type Float%20%28single-precision%29)))

(fn ConstructionScript
  (bind _rect_pool_x_size (Variables|RectangularPool|GetRect%20Pool%20X%20Size))
  (bind _rect_pool_y_size (Variables|RectangularPool|GetRect%20Pool%20Y%20Size))
  (bind _returnvalue (+ _rect_pool_y_size 4e+01))
  (bind _returnvalue_2 (+ _rect_pool_x_size 4e+01))
  (bind _returnvalue_3 (/ _returnvalue_2 1e+02))
  (bind _returnvalue_4 (/ _returnvalue 1e+02))
  (Utilities|FlowControl|Sequence
    (:then_0
      (CallFunction|AddRectangularMeshes))
    (:then_1
      ;[1 1 1] Add Bottom, Water
      (Utilities|FlowControl|Sequence
        (:then_0
          (bind _returnvalue_5 (AddComponent|AddStaticMeshComponent false (Math|Transform|MakeTransform (Math|Vector|MakeVector 0.0 0.0 (* (Variables|RectangularPool|GetDepth) -1.0)) (Math|Rotator|MakeRotator 0.0 0.0 0.0) (Math|Vector|MakeVector _returnvalue_3 _returnvalue_4 1.0))))
          (Rendering|Material|SetMaterial _returnvalue_5 0 (Variables|CopingandWalls|GetWalls%20Material)))
        (:then_1
          (if (Variables|Water|GetWater)
            (bind _returnvalue_6 (AddComponent|AddStaticMeshComponent false (Math|Transform|MakeTransform (Math|Vector|MakeVector 0.0 0.0 (Variables|Water|GetWater_Height)) "0, 0, 0" (Math|Vector|MakeVector _returnvalue_3 _returnvalue_4 1.0))))
            (Rendering|Material|SetMaterial _returnvalue_6 0 (Variables|Water|GetWater%20Material))))))
    (:then_2
      (CallFunction|AddLadders))))

(fn AddRectangularMeshes
  (bind _returnvalue (Math|Float|MakeLiteralFloat 1.0))
  (bind _coping_height (Variables|CopingandWalls|GetCoping%20Height))
  (bind _rectangular_pool_meshes_array (Variables|RectangularPool|GetRectangular%20Pool%20Meshes%20Array))
  (bind _rectangular_pool_meshes_array_2 (Variables|RectangularPool|GetRectangular%20Pool%20Meshes%20Array))
  (bind _rect_pool_y_size (Variables|RectangularPool|GetRect%20Pool%20Y%20Size))
  (bind _rect_pool_x_size (Variables|RectangularPool|GetRect%20Pool%20X%20Size))
  (bind _coping_height_2 (Variables|CopingandWalls|GetCoping%20Height))
  (bind _rect_pool_x_size_2 (Variables|RectangularPool|GetRect%20Pool%20X%20Size))
  (bind _rect_pool_y_size_2 (Variables|RectangularPool|GetRect%20Pool%20Y%20Size))
  (bind _coping_height_3 (Variables|CopingandWalls|GetCoping%20Height))
  (bind _rect_pool_y_size_3 (Variables|RectangularPool|GetRect%20Pool%20Y%20Size))
  (bind _rect_pool_x_size_3 (Variables|RectangularPool|GetRect%20Pool%20X%20Size))
  (bind _returnvalue_2 (/ _rect_pool_y_size_2 -2.0))
  (bind _returnvalue_3 (/ _rect_pool_x_size_3 -2.0))
  (bind _returnvalue_4 (- _rect_pool_x_size_2 0.2))
  (bind _returnvalue_5 (- _rect_pool_x_size_2 2e+02))
  (bind _returnvalue_6 (/ _rect_pool_x_size 2.0))
  (bind _returnvalue_7 (/ _rect_pool_y_size 2.0))
  (bind _returnvalue_8 (/ _rect_pool_x_size -2.0))
  (bind _returnvalue_9 (/ _rect_pool_y_size -2.0))
  (bind _returnvalue_10 (- _rect_pool_y_size_3 0.2))
  (bind _returnvalue_11 (- _rect_pool_y_size_3 2e+02))
  (bind _returnvalue_12 (/ _returnvalue_10 2e+02))
  (bind _returnvalue_13 (/ _returnvalue_4 2e+02))
  (bind _returnvalue_14 (Math|Float|Floor _returnvalue_13))
  (bind _returnvalue_15 (Math|Float|Floor _returnvalue_12))
  (bind _returnvalue_16 (* _returnvalue_15 2e+02))
  (bind _returnvalue_17 (* _returnvalue_14 2e+02))
  (bind _returnvalue_18 (/ _returnvalue_11 _returnvalue_16))
  (bind _returnvalue_19 (/ _returnvalue_5 _returnvalue_17))
  (Utilities|FlowControl|Sequence
    (:then_0
      ;[1 1 1] Add Corner Meshes
      (for _array_element (Utilities|Array|MakeArray (Math|Transform|MakeTransform (Math|Vector|MakeVector _returnvalue_8 _returnvalue_7 _coping_height) "0.000000,180.000000,0.000000" (Math|Vector|MakeVector _returnvalue 1.0 1.0)) (Math|Transform|MakeTransform (Math|Vector|MakeVector _returnvalue_8 _returnvalue_9 _coping_height) "0.000000,270.000000,0.000000" (Math|Vector|MakeVector 1.0 _returnvalue 1.0)) (Math|Transform|MakeTransform (Math|Vector|MakeVector _returnvalue_6 _returnvalue_9 _coping_height) "0, 0, 0" (Math|Vector|MakeVector _returnvalue 1.0 1.0)) (Math|Transform|MakeTransform (Math|Vector|MakeVector _returnvalue_6 _returnvalue_7 _coping_height) "0, 0, 0" (Math|Vector|MakeVector 1.0 -1.0 1.0)))
        (bind _returnvalue_20 (AddComponent|AddStaticMeshComponent false _array_element))
        (Utilities|Array|Add (Variables|RectangularPool|GetRectangular%20Pool%20Meshes%20Corners%20Array) _returnvalue_20)))
    (:then_1
      ;[1 1 1] Add X Meshes
      (for _index (range 0 (- _returnvalue_14 1))
        (bind _returnvalue_21 (AddComponent|AddStaticMeshComponent false (Math|Transform|MakeTransform (Math|Vector|MakeVector (+ (+ (/ (Variables|RectangularPool|GetRect%20Pool%20X%20Size) -2.0) 1e+02) (* (+ _index 0.5) (/ _returnvalue_5 _returnvalue_14))) _returnvalue_2 _coping_height_3) "0, 0, 0" (Math|Vector|MakeVector _returnvalue_19 1.0 1.0))))
        (bind _returnvalue_22 (AddComponent|AddStaticMeshComponent false (Math|Transform|MakeTransform (Math|Vector|MakeVector (+ (+ (/ (Variables|RectangularPool|GetRect%20Pool%20X%20Size) -2.0) 1e+02) (* (+ _index 0.5) (/ _returnvalue_5 _returnvalue_14))) (* _returnvalue_2 -1.0) _coping_height_3) "0.000000,180.000000,0.000000" (Math|Vector|MakeVector _returnvalue_19 1.0 1.0))))
        (Utilities|Array|Add _rectangular_pool_meshes_array _returnvalue_21)
        (Utilities|Array|Add _rectangular_pool_meshes_array _returnvalue_22)))
    (:then_2
      ;[1 1 1] Add Y Meshes
      (for _index_2 (range 0 (- _returnvalue_15 1))
        (bind _returnvalue_23 (AddComponent|AddStaticMeshComponent false (Math|Transform|MakeTransform (Math|Vector|MakeVector _returnvalue_3 (+ (+ (/ (Variables|RectangularPool|GetRect%20Pool%20Y%20Size) -2.0) 1e+02) (* (+ _index_2 0.5) (/ _returnvalue_11 _returnvalue_15))) _coping_height_2) "0.000000,270.000000,0.000000" (Math|Vector|MakeVector _returnvalue_18 1.0 1.0))))
        (Utilities|Array|Add _rectangular_pool_meshes_array_2 _returnvalue_23)
        (bind _returnvalue_24 (AddComponent|AddStaticMeshComponent false (Math|Transform|MakeTransform (Math|Vector|MakeVector (* _returnvalue_3 -1.0) (+ (+ (/ (Variables|RectangularPool|GetRect%20Pool%20Y%20Size) -2.0) 1e+02) (* (+ _index_2 0.5) (/ _returnvalue_11 _returnvalue_15))) _coping_height_2) "0.000000,90.000000,0.000000" (Math|Vector|MakeVector _returnvalue_18 1.0 1.0))))
        (Utilities|Array|Add _rectangular_pool_meshes_array_2 _returnvalue_24)))
    (:then_3
      ;[1 1 1] Customize
      (for _array_element_2 (Variables|RectangularPool|GetRectangular%20Pool%20Meshes%20Array)
        (Rendering|Material|SetMaterialbyName _array_element_2 "Wall" (Variables|CopingandWalls|GetWalls%20Material))
        (Rendering|Material|SetMaterialbyName _array_element_2 "Coping" (Variables|CopingandWalls|GetCoping%20Material)))
      (for _array_element_3 (Variables|RectangularPool|GetRectangular%20Pool%20Meshes%20Corners%20Array)
        (Rendering|Material|SetMaterialbyName _array_element_3 "Wall" (Variables|CopingandWalls|GetWalls%20Material))
        (Rendering|Material|SetMaterialbyName _array_element_3 "Coping" (Variables|CopingandWalls|GetCoping%20Material))))))

(fn AddLadders
  (Utilities|FlowControl|Sequence
    (:then_0
      (for _array_element (Variables|Ladders|GetLadder%20Positions)
        (bind _returnvalue (AddComponent|AddStaticMeshComponent false (Utilities|CalculateTransformAlongPoolEdge _array_element true)))
        ;[1 1 1] Select Ladder mesh depending on depth in this point
        (bind (_outhit _returnvalue_2) (Collision|LineTraceByChannel (+ (Transformation|GetWorldLocation _returnvalue) (* (Math|Vector|GetRightVector _returnvalue) 8e+01) "0.000000,0.000000,-50.000000") (+ (+ (Transformation|GetWorldLocation _returnvalue) (* (Math|Vector|GetRightVector _returnvalue) 8e+01) "0.000000,0.000000,-50.000000") "0.000000,0.000000,-200.000000") "TraceTypeQuery1" false 0 "None" false "(R=1.000000,G=0.000000,B=0.000000,A=1.000000)" "(R=0.000000,G=1.000000,B=0.000000,A=1.000000)" 4.0))
        (if _returnvalue_2
          (if (> (.z (- (Transformation|GetActorLocation) (.location _outhit))) 1.5e+02)
            (Components|StaticMesh|SetStaticMesh _returnvalue "/Game/Water_Slide_System/Meshes/Pool/SM_Ladder_5_Steps.SM_Ladder_5_Steps")
            (elif (< (.z (- (Transformation|GetActorLocation) (.location _outhit))) 1.2e+02)
              (Components|StaticMesh|SetStaticMesh _returnvalue "/Game/Water_Slide_System/Meshes/Pool/SM_Ladder_3_Steps.SM_Ladder_3_Steps"))))))))