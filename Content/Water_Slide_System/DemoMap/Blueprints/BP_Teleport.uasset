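; BP_Teleport is a one-way teleporter pad for the water slide demo map, acting as either sender or receiver via IsReceiver.
; A pawn entering a sender's sphere triggers a sound, then after a short delay moves above the linked Receiver, and player 0's view yaw is realigned.
; A timeline flashes both pads' lights, while senders also pulse on a sine wave.
; Construction removes the receiver's sphere and makes senders inherit their receiver's color.
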(event OnComponentBeginOverlap(Sphere)
  (params (OverlappedComponent :type Primitive%20Component%20Object%20Reference) (OtherActor :type Actor%20Object%20Reference) (OtherComp :type Primitive%20Component%20Object%20Reference) (OtherBodyIndex :type Integer) (bFromSweep :type Boolean) (SweepResult :type Hit%20Result%20Structure%20%28by%20ref%29))
  (bind _receiver (Variables|Teleport|GetReceiver))
  (bind _defaultsceneroot (Variables|BP_Teleport_C|GetDefaultSceneRoot _receiver))
  (bind _returnvalue (Transformation|GetWorldTransform _defaultsceneroot))
  (if (Utilities|Enum|Equal(Enum) (Collision|GetCollisionObjectType OtherComp) "ECC_Pawn")
    (if (not (Variables|Teleport|GetIs%20Receiver))
      (Utilities|IsValid (Variables|Teleport|GetReceiver)
        (:Is%20Valid
          (Audio|PlaySound2D "/Game/Water_Slide_System/DemoMap/Sound/S_Teleport.S_Teleport" 1.5 1.0 0.0 0 0)
          (Utilities|FlowControl|Sequence
            (:then_0
              (Utilities|FlowControl|Delay 0.9)
              (Transformation|SetActorLocation OtherActor (+ (.location _returnvalue) "0.000000,0.000000,100.000000") false false)
              (Pawn|SetControlRotation (Game|GetPlayerController 0) (Math|Rotator|MakeRotator 0.0 0.0 (+ (.yaw (.rotation _returnvalue)) 9e+01))))
            (:then_1
              (bind _newtrack_0 (Timeline|Light%20Intensity PlayFromStart)
                (:Update
                  (Variables|Teleport|SetFunctioning%20Intensity (* _newtrack_0 9e+01))
                  (Variables|BP_Teleport_C|SetFunctioning%20Intensity (Variables|Teleport|GetReceiver) (* _newtrack_0 9e+01)))))))))))

(event EventTick
  (params (DeltaSeconds :type Float%20%28single-precision%29))
  (Rendering|Components|Light|SetIntensity (Variables|Default|GetPointLight) (+ (Variables|Teleport|GetFunctioning%20Intensity) (Math|Float|SelectFloat 0.0 (* (+ (Math|Trig|Sin(Radians) (Utilities|Time|GetRealTimeSeconds)) 2.0) 3e+02) (Variables|Teleport|GetIs%20Receiver)))))

(fn ConstructionScript
  (Utilities|FlowControl|Sequence
    (:then_1
      (if (Variables|Teleport|GetIs%20Receiver)
        (Rendering|Components|Light|SetIntensity (Variables|Default|GetPointLight) 0.0)
        (Components|DestroyComponent (Variables|Default|GetSphere))
        (else
          (Rendering|Material|SetScalarParameterValueonMaterials (Variables|Default|GetSM_Teleport) "Emissive Tiilng" -2.0)
          (Variables|Teleport|SetColor (Math|Conversions|ToColor(LinearColor) (Math|Color|SelectColor (Math|Conversions|ToLinearColor(Color) (Variables|BP_Teleport_C|GetColor (Variables|Teleport|GetReceiver))) "(R=0.000000,G=0.000000,B=0.000000,A=1.000000)" (Utilities|IsValid (Variables|Teleport|GetReceiver))))))))
    (:then_2
      (Rendering|Material|SetVectorParameterValueonMaterials (Variables|Default|GetSM_Teleport) "Emissive Color" (Math|Conversions|ToVector(LinearColor) (Math|Conversions|ToLinearColor(Color) (Variables|Teleport|GetColor))))
      (Rendering|Components|Light|SetLightColor (Variables|Default|GetPointLight) (Math|Conversions|ToLinearColor(Color) (Variables|Teleport|GetColor)) false))))